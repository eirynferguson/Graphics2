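; BP_Button is a pressure-style button that activates linked actors while anything overlaps its sphere trigger.
; Each overlap swaps the dynamic material to pressed colour, emissive and a WPO offset, and sends ActivateMessage through BPI_Activate to every actor in ActorsToActivate.
; It tracks overlapping actors, so only when the last one leaves does it reset the visuals and send DeactivateMessage.
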(event `self.ReceiveBeginPlay`
  (bind _returnvalue (`PrimitiveComponent.CreateDynamicMaterialInstance` (`self.Button`) 0 "/Game/MyWork/Materials/M_Button_Inst.M_Button_Inst" "None"))
  (set `self.ButtonMat` _returnvalue))

(event `self.Sphere.OnComponentBeginOverlap`
  (params (OverlappedComponent :type "PrimitiveComponent Object Reference") (OtherActor :type "Actor Object Reference") (OtherComp :type "PrimitiveComponent Object Reference") (OtherBodyIndex :type Integer) (bFromSweep :type Boolean) (SweepResult :type "HitResult Structure (by ref)"))
  (`KismetArrayLibrary.Array_AddUnique` (`self.Overlapping Actors`) OtherActor)
  (`self.ShowHighlightVisuals`)
  (for _array_element (`self.ActorsToActivate`)
    (if (`KismetSystemLibrary.DoesImplementInterface` _array_element "/Game/MyWork/Blueprint/BPI_Activate.BPI_Activate_C")
      (message `/Game/MyWork/Blueprint/BPI_Activate.Activate` _array_element))))

(event `self.Sphere.OnComponentEndOverlap`
  (params (OverlappedComponent :type "PrimitiveComponent Object Reference") (OtherActor :type "Actor Object Reference") (OtherComp :type "PrimitiveComponent Object Reference") (OtherBodyIndex :type Integer))
  (bind _overlapping_actors (`self.Overlapping Actors`))
  (`KismetArrayLibrary.Array_RemoveItem` _overlapping_actors OtherActor)
  (if (== (`KismetArrayLibrary.Array_Length` _overlapping_actors) 0)
    (`self.ResetButtonVisuals`)
    (for _array_element (`self.ActorsToActivate`)
      (if (`KismetSystemLibrary.DoesImplementInterface` _array_element "/Game/MyWork/Blueprint/BPI_Activate.BPI_Activate_C")
        (message `/Game/MyWork/Blueprint/BPI_Activate.Deactivate` _array_element)))))

(fn `ResetButtonVisuals`
  (bind _buttonmat (`self.ButtonMat`))
  (`MaterialInstanceDynamic.SetVectorParameterValue` _buttonmat "Colour" (`self.ButtonColour`))
  (`MaterialInstanceDynamic.SetVectorParameterValue` :`self` _buttonmat :`ParameterName` "WPO")
  (`MaterialInstanceDynamic.SetVectorParameterValue` :`self` _buttonmat :`ParameterName` "Emissive"))

(fn `ShowHighlightVisuals`
  (bind _buttonmat (`self.ButtonMat`))
  (`MaterialInstanceDynamic.SetVectorParameterValue` _buttonmat "Colour" (`self.ButtonPressedColour`))
  (`MaterialInstanceDynamic.SetVectorParameterValue` _buttonmat "WPO" (`self.ButtonOffSetColour`))
  (`MaterialInstanceDynamic.SetVectorParameterValue` _buttonmat "Emissive" (`self.ButtonEmissiveColour`)))

(fn `UserConstructionScript`)