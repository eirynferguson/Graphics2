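; Actor component that smoothly turns its owning actor to face a target actor.
; Each tick, while TargetActor is valid, it builds a rotation from the direction between the owner and the target.
; It then interpolates the owner's rotation toward it with RInterpTo at RotateSpeed, affecting all axes rather than yaw alone.
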(event `self.ReceiveTick`
  (params (DeltaSeconds :type "Float (single-precision)"))
  (bind _returnvalue (`self.GetOwner`))
  (bind _targetactor (`self.TargetActor`))
  (`/Engine/EditorBlueprintResources/StandardMacros.IsValid` _targetactor
    (:`Is Valid`
      (`Actor.K2_SetActorRotation` _returnvalue (`KismetMathLibrary.RInterpTo` (`Actor.K2_GetActorRotation` _returnvalue) (`KismetMathLibrary.Conv_VectorToRotator` (- (`Actor.K2_GetActorLocation` _targetactor) (`Actor.K2_GetActorLocation` (`self.GetOwner`)))) DeltaSeconds (`self.RotateSpeed`)) false))))