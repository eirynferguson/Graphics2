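; MoveForward is an actor component that pushes its owning actor along its forward vector once movement is activated.
; ActivateMovement sets the CanMove flag, and the file has no logic to clear it.
; While the flag is set, Tick offsets the owner's location by Speed scaled by delta time, without sweeping, so the move ignores blocking collision.
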(event `self.ReceiveTick`
  (params (DeltaSeconds :type "Float (single-precision)"))
  (bind _returnvalue (`self.GetOwner`))
  (if (`self.CanMove`)
    (`Actor.K2_SetActorLocation` _returnvalue (+ (* (* DeltaSeconds (`self.Speed`)) (`Actor.GetActorForwardVector` _returnvalue)) (`Actor.K2_GetActorLocation` _returnvalue)) false false)))

(event `ActivateMovement`
  (set `self.CanMove` true))