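; Actor component that smoothly turns its owning actor to face a TargetActor.
; Each Tick, while TargetActor is valid, it computes a look-at rotation toward the target's position flattened to the owner's height, limiting the turn to yaw.
; It interpolates from the current rotation with RInterpTo at RotateSpeed and applies the result to the owner.
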(event `self.ReceiveTick`
  (params (DeltaSeconds :type "Float (single-precision)"))
  (bind _returnvalue (`self.GetOwner`))
  (bind _targetactor (`self.TargetActor`))
  (bind (_returnvalue_x _returnvalue_y) (`KismetMathLibrary.BreakVector` (`Actor.K2_GetActorLocation` _targetactor)))
  (bind (_returnvalue_x_2 _returnvalue_y_2 _returnvalue_z) (`KismetMathLibrary.BreakVector` (`Actor.K2_GetActorLocation` (`self.GetOwner`))))
  (`/Engine/EditorBlueprintResources/StandardMacros.IsValid` _targetactor
    (:`Is Valid`
      (`Actor.K2_SetActorRotation` _returnvalue (`KismetMathLibrary.RInterpTo` (`Actor.K2_GetActorRotation` _returnvalue) (`KismetMathLibrary.FindLookAtRotation` (`KismetMathLibrary.MakeVector` _returnvalue_x_2 _returnvalue_y_2 _returnvalue_z) (`KismetMathLibrary.MakeVector` _returnvalue_x _returnvalue_y _returnvalue_z)) DeltaSeconds (`self.RotateSpeed`)) false))))